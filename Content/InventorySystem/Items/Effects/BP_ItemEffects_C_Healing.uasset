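; Consumable item effect actor that heals the player as soon as it spawns.
; On BeginPlay it casts player character 0 to BP_Player, calls its own InteractWith event, then destroys itself.
; InteractWith passes the Amount variable to Healing on the player's health component.
; LookAt returns an empty string, so it supplies no look-at text.
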(event EventBeginPlay
  (bind _returnvalue (Game|GetPlayerCharacter 0))
  (Utilities|IsValid _returnvalue
    (:Is%20Valid
      (bind _asbp_player (Utilities|Casting|CastToBP_Player _returnvalue))
      (CallFunction|Interactwith _asbp_player)
      (Actor|DestroyActor))))

(event EventInteractwith
  (params (PlayerCharacter :type BP%20Player%20Object%20Reference))
  (Default|Healing (Variables|/Game/BP_Logic/BP_Player/BP_Player.BP_Player_C|GetBPC_HealthComponent PlayerCharacter) (Variables|Default|GetAmount)))

(fn ConstructionScript
  (|CallParentFunction))

(fn Lookat
  (return ""))