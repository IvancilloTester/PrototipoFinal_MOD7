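; Player stats component for BP_Player that tracks health and stamina and mirrors them on the HUD progress bars.
; On BeginPlay it waits one tick, caches the owning BP_Player and initializes both bars.
; Decrease functions subtract, update the bar and return true once the stat is depleted, leaving the response to the caller.
; Increase functions add and refresh the bar without clamping to the maximum.
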(event EventBeginPlay
  (Utilities|FlowControl|DelayUntilNextTick)
  (bind _asbp_player (Utilities|Casting|CastToBP_Player (Components|GetOwner)))
  (Variables|Default|SetOwner_Player_Character _asbp_player)
  (Progress|SetPercent (Variables|/Game/BluePrints/BP_UIs/WBP_HUD.WBP_HUD_C|GetStamina_Bar (Variables|/Game/BluePrints/BP_Player_Enemies_Assets/BP_Player.BP_Player_C|GetHUD_Widget (Variables|Default|GetOwner_Player_Character))) (/ (Variables|Stamina|GetCurrentStamina) (Variables|Stamina|GetMaxStamina)))
  (Progress|SetPercent (Variables|/Game/BluePrints/BP_UIs/WBP_HUD.WBP_HUD_C|GetHealth_Bar (Variables|/Game/BluePrints/BP_Player_Enemies_Assets/BP_Player.BP_Player_C|GetHUD_Widget (Variables|Default|GetOwner_Player_Character))) (/ (Variables|Health|GetCurrentHealth) (Variables|Health|GetMaxHealth))))

(fn DecreaseHealth
  (params (Damage :type Float%20%28double-precision%29))
  ;[0.15 0.15 0.15 0.5] Health_Logic
  (if (not (<= (Variables|Health|GetCurrentHealth) 0.0))
    (Variables|Health|SetCurrentHealth (- (Variables|Health|GetCurrentHealth) Damage))
    (Progress|SetPercent (Variables|/Game/BluePrints/BP_UIs/WBP_HUD.WBP_HUD_C|GetHealth_Bar (Variables|/Game/BluePrints/BP_Player_Enemies_Assets/BP_Player.BP_Player_C|GetHUD_Widget (Variables|Default|GetOwner_Player_Character))) (/ (Variables|Health|GetCurrentHealth) (Variables|Health|GetMaxHealth)))
    ;[0.15 0.15 0.15 0.5] Death_Logic
    (if (<= (Variables|Health|GetCurrentHealth) 0.0)
      _
      (else
        (return false))))
  (return true))

(fn IncreaseHealth
  (params (HealingValue :type Float%20%28double-precision%29))
  ;[0.15 0.15 0.15 0.5] Healing_Logic_(Objetos curativos?)
  (Variables|Health|SetCurrentHealth (+ HealingValue (Variables|Health|GetCurrentHealth)))
  (Progress|SetPercent (Variables|/Game/BluePrints/BP_UIs/WBP_HUD.WBP_HUD_C|GetHealth_Bar (Variables|/Game/BluePrints/BP_Player_Enemies_Assets/BP_Player.BP_Player_C|GetHUD_Widget (Variables|Default|GetOwner_Player_Character))) (/ (Variables|Health|GetCurrentHealth) (Variables|Health|GetMaxHealth))))

(fn DecreaseStamina
  (params (DecreasedStamina :type Float%20%28double-precision%29))
  ;[0.15 0.15 0.15 0.5] Decreasing_Stamina_Logic
  (if (not (<= (Variables|Stamina|GetCurrentStamina) 0.0))
    (Variables|Stamina|SetCurrentStamina (- (Variables|Stamina|GetCurrentStamina) DecreasedStamina))
    (Progress|SetPercent (Variables|/Game/BluePrints/BP_UIs/WBP_HUD.WBP_HUD_C|GetStamina_Bar (Variables|/Game/BluePrints/BP_Player_Enemies_Assets/BP_Player.BP_Player_C|GetHUD_Widget (Variables|Default|GetOwner_Player_Character))) (/ (Variables|Stamina|GetCurrentStamina) (Variables|Stamina|GetMaxStamina)))
    ;[0.15 0.15 0.15 0.5] Player_Death_Logic
    (if (<= (Variables|Stamina|GetCurrentStamina) 0.0)
      _
      (else
        (return false))))
  (return true))

(fn IncreaseStamina
  (params (AddedStamina :type Float%20%28double-precision%29))
  ;[0.15 0.15 0.15 0.5] Increasing_Stamina_Logic
  (Variables|Stamina|SetCurrentStamina (+ (Variables|Stamina|GetCurrentStamina) AddedStamina))
  (Progress|SetPercent (Variables|/Game/BluePrints/BP_UIs/WBP_HUD.WBP_HUD_C|GetStamina_Bar (Variables|/Game/BluePrints/BP_Player_Enemies_Assets/BP_Player.BP_Player_C|GetHUD_Widget (Variables|Default|GetOwner_Player_Character))) (/ (Variables|Stamina|GetCurrentStamina) (Variables|Stamina|GetMaxStamina))))