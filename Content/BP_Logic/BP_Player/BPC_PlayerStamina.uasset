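; Player stamina component that tracks current stamina against a maximum through two functions.
; DecreaseStamina subtracts the given amount while stamina is above zero and returns whether it is depleted.
; IncreaseStamina adds the given amount only while stamina is below the maximum.
; Neither function clamps the result, so stamina can pass zero or the maximum.
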(fn DecreaseStamina
  (params (DecreasedStamina :type Float%20%28double-precision%29))
  ;[0.15 0.15 0.15 0.5] Decreasing_Stamina_Logic
  (if (not (<= (Variables|Stamina|GetCurrentStamina) 0.0))
    (Variables|Stamina|SetCurrentStamina (- (Variables|Stamina|GetCurrentStamina) DecreasedStamina))
    (if (<= (Variables|Stamina|GetCurrentStamina) 0.0)
      _
      (else
        (return false))))
  (return true))

(fn IncreaseStamina
  (params (AddedStamina :type Float%20%28double-precision%29))
  ;[0.15 0.15 0.15 0.5] Increasing_Stamina_Logic
  (if (< (Variables|Stamina|GetCurrentStamina) (Variables|Stamina|GetMaxStamina))
    (Variables|Stamina|SetCurrentStamina (+ (Variables|Stamina|GetCurrentStamina) AddedStamina))
    (if (== (Variables|Stamina|GetCurrentStamina) (Variables|Stamina|GetMaxStamina))
      (return))))