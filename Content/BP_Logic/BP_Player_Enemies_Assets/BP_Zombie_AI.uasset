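; Zombie enemy Blueprint that carries a health component, a floating health bar and a montage-based attack.
; On BeginPlay it hides the health bar and passes its health component to the zombie HUD widget.
; A sphere trigger shows the bar while the player overlaps it and hides it when they leave.
; An Attack function plays the zombie attack montage and returns the PlayAnimMontage result.
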(event OnComponentBeginOverlap(Sphere)
  (params (OverlappedComponent :type Primitive%20Component%20Object%20Reference) (OtherActor :type Actor%20Object%20Reference) (OtherComp :type Primitive%20Component%20Object%20Reference) (OtherBodyIndex :type Integer) (bFromSweep :type Boolean) (SweepResult :type Hit%20Result%20Structure%20%28by%20ref%29))
  (Utilities|Casting|CastToBP_Player OtherActor)
  (Rendering|SetVisibility (Variables|Default|GetHealth_BarHUD) true false))

(event OnComponentEndOverlap(Sphere)
  (params (OverlappedComponent :type Primitive%20Component%20Object%20Reference) (OtherActor :type Actor%20Object%20Reference) (OtherComp :type Primitive%20Component%20Object%20Reference) (OtherBodyIndex :type Integer))
  (Utilities|Casting|CastToBP_Player OtherActor)
  (Rendering|SetVisibility (Variables|Default|GetHealth_BarHUD) false false))

(event EventBeginPlay
  (bind _health_barhud (Variables|Default|GetHealth_BarHUD))
  (Rendering|SetVisibility _health_barhud false false)
  (bind _aswbp_zombie_hud (Utilities|Casting|CastToWBP_ZombieHUD (UserInterface|GetWidget _health_barhud)))
  (Variables|/Game/BP_Logic/BP_UIs/WBP_ZombieHUD.WBP_ZombieHUD_C|SetHealthComp _aswbp_zombie_hud (Variables|Default|GetBPC_HealthComponent)))

(fn ConstructionScript)

(fn Attack
  (bind _returnvalue (Animation|PlayAnimMontage "/Game/BP_Anim/Zombie_SkeletalMesh/Zombie_Attack_Montage.Zombie_Attack_Montage" 1.0 "None"))
  (return _returnvalue))