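; Big zombie enemy that runs a behavior tree, attacks via montage and drops loot when killed.
; BeginPlay links the health component to a widget health bar, shown while the player overlaps its sphere, and hands the tree to BP_AIController_B.
; Death plays a dying animation, drops a random apple, energy item or batch of bullets at a downward-traced point, then destroys the actor after a delay.
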(event OnComponentBeginOverlap(Sphere)
  (params (OverlappedComponent :type Primitive%20Component%20Object%20Reference) (OtherActor :type Actor%20Object%20Reference) (OtherComp :type Primitive%20Component%20Object%20Reference) (OtherBodyIndex :type Integer) (bFromSweep :type Boolean) (SweepResult :type Hit%20Result%20Structure%20%28by%20ref%29))
  (Utilities|Casting|CastToBP_Player OtherActor)
  (Rendering|SetVisibility (Variables|Default|GetHealth_BarHUD) true false))

(event OnComponentEndOverlap(Sphere)
  (params (OverlappedComponent :type Primitive%20Component%20Object%20Reference) (OtherActor :type Actor%20Object%20Reference) (OtherComp :type Primitive%20Component%20Object%20Reference) (OtherBodyIndex :type Integer))
  (Utilities|Casting|CastToBP_Player OtherActor)
  (Rendering|SetVisibility (Variables|Default|GetHealth_BarHUD) false false))

(event Custom|DropLoot
  (bind _returnvalue (Math|Random|RandomInteger 5))
  (bind _returnvalue_2 (Transformation|GetActorLocation))
  (bind _returnvalue_3 (Utilities|Select :Index _returnvalue :Option%200 "/Game/InventorySystem/Items/BP_ItemBase_C_Apple.BP_ItemBase_C_Apple_C" :Option%201 "/Game/InventorySystem/Items/BP_ItemBase_C_Energy.BP_ItemBase_C_Energy_C" :Option%202 "/Game/InventorySystem/Items/BP_ItemBase_C_Bullet.BP_ItemBase_C_Bullet_C" :Option%203 "/Game/InventorySystem/Items/BP_ItemBase_C_Apple.BP_ItemBase_C_Apple_C" :Option%204 "/Game/InventorySystem/Items/BP_ItemBase_C_Apple.BP_ItemBase_C_Apple_C"))
  ;[0.15 0.15 0.15 0.5] LOOT
  (bind _outhit (Collision|LineTraceByChannel _returnvalue_2 (+ _returnvalue_2 "0.000000,0.000000,-200.000000") "TraceTypeQuery1" false (Utilities|Array|MakeArray (Game|GetPlayerCharacter 0)) "None"))
  (if (not (== _returnvalue_3 "/Game/InventorySystem/Items/BP_ItemBase_C_Bullet.BP_ItemBase_C_Bullet_C"))
    (Game|SpawnActorfromClass _returnvalue_3 (Math|Transform|MakeTransform (.Location (Collision|BreakHitResult _outhit)) (Math|Rotator|MakeRotator 0.0 0.0 (Math|Random|RandomFloatinRange 0.0 3.6e+02))) "Undefined" "MultiplyWithRoot" 0 0)
    (Development|PrintString "Dropped Loot!" true true "(R=1.000000,G=0.000000,B=0.827856,A=1.000000)")
    (else
      (while (< (Variables|Default|GetBulletsGranted) 4)
        (Game|SpawnActorfromClass "/Game/InventorySystem/Items/BP_ItemBase_C_Bullet.BP_ItemBase_C_Bullet_C" (Math|Transform|MakeTransform (.Location (Collision|BreakHitResult _outhit)) (Math|Rotator|MakeRotator 0.0 0.0 (Math|Random|RandomFloatinRange 0.0 3.6e+02))) "Undefined" "MultiplyWithRoot" 0 0)
        (Variables|Default|SetBulletsGranted (+ (stale _output_get) 1))
        (Development|PrintString "Droped Bullets!!" true true "(R=1.000000,G=0.343636,B=0.000000,A=1.000000)"))
      (bind _output_get (Variables|Default|SetBulletsGranted 0)))))

(event Custom|Death_Event
  (CallFunction|Death true)
  (Utilities|FlowControl|Delay 4.0)
  (Actor|DestroyActor))

(event EventBeginPlay
  (bind _health_barhud (Variables|Default|GetHealth_BarHUD))
  (Rendering|SetVisibility _health_barhud false false)
  (bind _aswbp_zombie_hud (Utilities|Casting|CastToWBP_ZombieHUD (UserInterface|GetWidget _health_barhud)))
  (Variables|/Game/BP_Logic/BP_UIs/WBP_ZombieHUD.WBP_ZombieHUD_C|SetHealthComp _aswbp_zombie_hud (Variables|Default|GetBPC_HealthComponent))
  (bind _asbp_aicontroller_b (Utilities|Casting|CastToBP_AIController_B (AI|GetAIController self)))
  (Default|SetBTEvent _asbp_aicontroller_b (Variables|Default|GetmyBT))
  (EventDispatchers|AssignDeath (Variables|Default|GetBPC_HealthComponent) (delegate Custom|Death_Event)))

(fn ConstructionScript)

(fn Death
  (params (IsDead :type Boolean))
  (Variables|Default|SetIsDead IsDead)
  (Components|Animation|PlayAnimation (Variables|Character|GetMesh) "/Game/BP_Anim/ZombieBig_SkeletalMesh/ZombiBig_Dying.ZombiBig_Dying" false)
  (CallFunction|DropLoot))

(fn Attack
  (bind _returnvalue (Animation|PlayAnimMontage "/Game/BP_Anim/Zombie_SkeletalMesh/Zombie_Attack_Montage.Zombie_Attack_Montage" 1.0 "None"))
  (return _returnvalue))