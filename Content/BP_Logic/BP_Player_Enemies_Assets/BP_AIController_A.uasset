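; AI controller that runs a supplied behavior tree and feeds it a target actor from perception for detecting and chasing.
; SetBT_Event starts the given tree when it is valid.
; Perception updates write a successfully sighted actor to the TargetActor_Key blackboard entry.
; Lost sight, or an update from any other sense, clears that key.
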(event OnTargetPerceptionUpdated(AIPerception)
  (params (Actor :type Actor%20Object%20Reference) (Stimulus :type AI%20Stimulus%20Structure))
  ;[0.15 0.15 0.15 0.5] Detect_And_Chase_Player
  (bind _returnvalue (Class|AIPerceptionSystem|GetSenseClassforStimulus Stimulus))
  (if (== _returnvalue "/Script/AIModule.AISense_Sight")
    (if (.bSuccessfullySensed (Utilities|Struct|BreakAIStimulus Stimulus))
      (AI|Components|Blackboard|SetValueasObject (AI|GetBlackboard 0) (Utilities|Name|MakeLiteralName "TargetActor_Key") Actor)
      (else
        (AI|Components|Blackboard|SetValueasObject (AI|GetBlackboard 0) (Utilities|Name|MakeLiteralName "TargetActor_Key") 0 :!label _label)))
    (else
      (goto _label))))

(event Custom|SetBT_Event
  (params (NewBT :type Behavior%20Tree%20Object%20Reference))
  (Utilities|IsValid NewBT
    (:Is%20Valid
      (AI|RunBehaviorTree NewBT))))

(fn ConstructionScript)