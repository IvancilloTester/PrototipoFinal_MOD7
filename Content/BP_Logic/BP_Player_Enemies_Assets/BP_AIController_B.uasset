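; AI controller that runs behavior trees and tracks a sighted target through AI perception.
; A custom event starts whichever valid behavior tree it is given.
; Perception updates write a successfully sensed sight actor to the ActorTarget_Key blackboard entry, with no filtering by actor type.
; Lost sight, or an update from any other sense, clears that entry.
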(event OnTargetPerceptionUpdated(AIPerception)
  (params (Actor :type Actor%20Object%20Reference) (Stimulus :type AI%20Stimulus%20Structure))
  (bind _returnvalue (Class|AIPerceptionSystem|GetSenseClassforStimulus Stimulus))
  (if (== _returnvalue "/Script/AIModule.AISense_Sight")
    (if (.bSuccessfullySensed (Utilities|Struct|BreakAIStimulus Stimulus))
      (AI|Components|Blackboard|SetValueasObject (AI|GetBlackboard 0) (Utilities|Name|MakeLiteralName "ActorTarget_Key") Actor)
      (else
        (AI|Components|Blackboard|SetValueasObject (AI|GetBlackboard 0) (Utilities|Name|MakeLiteralName "ActorTarget_Key") 0 :!label _label)))
    (else
      (goto _label))))

(event Custom|SetBT_Event
  (params (NewBT :type Behavior%20Tree%20Object%20Reference))
  (Utilities|IsValid NewBT
    (:Is%20Valid
      (AI|RunBehaviorTree NewBT))))

(fn ConstructionScript)