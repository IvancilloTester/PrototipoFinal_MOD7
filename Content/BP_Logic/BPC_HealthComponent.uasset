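; BPC_HealthComponent is a health component that tracks current health and death state through Damage and Healing functions.
; Damage subtracts from CurrentHealth, clamping at zero and setting IsDead on a lethal hit, and prints the remaining health otherwise.
; Healing adds to CurrentHealth up to MaxHealth.
; Both functions do nothing once IsDead is set, and death only sets that flag without firing any event.
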(fn Damage
  (params (Damage :type Float%20%28double-precision%29))
  (if (not (Variables|Default|GetIsDead))
    (if (<= (- (Variables|Default|GetCurrentHealth) Damage) 0.0)
      (Variables|Default|SetCurrentHealth 0.0)
      (Variables|Default|SetIsDead true)
      (else
        (bind _output_get (Variables|Default|SetCurrentHealth (- (Variables|Default|GetCurrentHealth) Damage)))
        (Development|PrintString (Utilities|String|ToString(Float) _output_get))))))

(fn Healing
  (params (Heal :type Float%20%28double-precision%29))
  (if (not (Variables|Default|GetIsDead))
    (if (>= (+ (Variables|Default|GetCurrentHealth) Heal) (Variables|Default|GetMaxHealth))
      (Variables|Default|SetCurrentHealth (Variables|Default|GetMaxHealth))
      (else
        (Variables|Default|SetCurrentHealth (+ (Variables|Default|GetCurrentHealth) Heal))))))