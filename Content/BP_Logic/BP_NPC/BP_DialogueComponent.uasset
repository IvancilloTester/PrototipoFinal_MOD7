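; Actor component that runs dialogue between a player and an NPC, with both sides carrying the same component.
; On BeginPlay, it hands its dialogue tree to the owner's AIC_NPC controller.
; Begin, Advance and End track talking state and partner; the player side, identified by lacking that controller on begin, forwards calls to the partner's component.
; The NPC side starts and advances the tree through its controller and stops brain logic on end.
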(event EventBeginPlay
  (bind _asaic_npc (Utilities|Casting|CastToAIC_NPC (AI|GetAIController (Components|GetOwner))))
  (Variables|/Game/BP_Logic/BP_NPC/AIC_NPC.AIC_NPC_C|SetBP_DialogTrigger _asaic_npc (Variables|Default|GetMyDialogueTree)))

(fn BeginDialogue
  (params (ActorIn :type Actor%20Object%20Reference))
  (bind _returnvalue (Components|GetOwner))
  ;[0 0.07219 0.15 0.5] Begin Dialogue with an NPC while not talking to another NPC
  ;;[1 1 1 0.5] Logica de diálogo inicial
  (if (and (Utilities|IsValid (Actor|GetComponentbyClass ActorIn "BP_DialogueComponent_C")) (not (Variables|Default|GetIsTalking)))
    ;;[0.9073 0.9073 0.9073 0.5] Mientras hablo guardo con quien estoy hablando
    (Variables|Default|SetIsTalking true)
    (Variables|Default|SetOtherActor ActorIn)
    (bind _asaic_npc (Utilities|Casting|CastToAIC_NPC (AI|GetAIController _returnvalue))
      (:then
        (Default|AIBeginDialogueTree _asaic_npc)
        (Variables|Default|SetIsPlayer false))
      (:CastFailed
        (CallFunction|BeginDialogue (Actor|GetComponentbyClass (Variables|Default|GetOtherActor) "BP_DialogueComponent_C") _returnvalue)
        (Variables|Default|SetIsPlayer true)))))

(fn EndDialogue
  (params (ActorIn :type Actor%20Object%20Reference))
  (bind _returnvalue (Actor|GetComponentbyClass ActorIn "BP_DialogueComponent_C"))
  ;[0.008379 0.05096 0.15 0.5] Ending dialogue after talking to an NPC
  ;;[0.9156 0.9156 0.9156 0.5] Cuando hay dialogo y SI esta hablando
  (if (and (Utilities|IsValid _returnvalue) (Variables|Default|GetIsTalking))
    ;;[0.874 0.874 0.874 0.5] Hablando
    (Variables|Default|SetIsTalking false)
    (Variables|Default|SetOtherActor 0)
    ;;[0.8906 0.8906 0.8906 0.5] Si no soy el player
    (if (not (Variables|Default|GetIsPlayer))
      ;;[0.8906 0.8906 0.8906 0.5] Paramos el BT
      (AI|Logic|StopLogic (Variables|/Script/AIModule.AIController|GetBrainComponent (AI|GetAIController (Components|GetOwner))) "")
      (else
        ;;[0.9031 0.9031 0.9031 0.5] Pido al NPC que pare
        (CallFunction|EndDialogue _returnvalue (Components|GetOwner))))))

(fn AdvanceDialogue
  (bind _otheractor (Variables|Default|GetOtherActor))
  (bind _returnvalue (Actor|GetComponentbyClass _otheractor "BP_DialogueComponent_C"))
  ;[0.8781 0.8781 0.8781 0.5] Si estoy hablando
  (if (Variables|Default|GetIsTalking)
    ;[0.8656 0.8656 0.8656 0.5] Si soy el jugador
    (if (Variables|Default|GetIsPlayer)
      ;[0.899 0.899 0.899 0.5] Pido que avance el dialogo
      (Utilities|IsValid _otheractor
        (:Is%20Valid
          (Utilities|IsValid _returnvalue
            (:Is%20Valid
              (CallFunction|AdvanceDialogue _returnvalue)))))
      (else
        ;[0.9156 0.9156 0.9156 0.5] NPC avanza el dialogo
        (bind _asaic_npc (Utilities|Casting|CastToAIC_NPC (AI|GetAIController (Components|GetOwner))))
        (Default|AIAdvanceDialogueTree _asaic_npc)))))