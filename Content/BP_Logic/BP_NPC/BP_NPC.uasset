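; BP_NPC is an NPC Blueprint that starts and ends dialogue based on proximity.
; When another actor enters its Dialog_Box, the NPC looks for a BP_DialogueComponent on that actor and calls BeginDialogue with itself as the argument.
; Leaving the box calls EndDialogue the same way, so the overlapping actor's component handles the conversation and the NPC only triggers it.
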(event OnComponentBeginOverlap(Dialog_Box)
  (params (OverlappedComponent :type Primitive%20Component%20Object%20Reference) (OtherActor :type Actor%20Object%20Reference) (OtherComp :type Primitive%20Component%20Object%20Reference) (OtherBodyIndex :type Integer) (bFromSweep :type Boolean) (SweepResult :type Hit%20Result%20Structure%20%28by%20ref%29))
  (bind _returnvalue (Actor|GetComponentbyClass OtherActor "/Game/BP_Logic/BP_NPC/BP_DialogueComponent.BP_DialogueComponent_C"))
  (if (!= OtherActor self)
    (Utilities|IsValid _returnvalue
      (:Is%20Valid
        (Default|BeginDialogue _returnvalue self)))))

(event OnComponentEndOverlap(Dialog_Box)
  (params (OverlappedComponent :type Primitive%20Component%20Object%20Reference) (OtherActor :type Actor%20Object%20Reference) (OtherComp :type Primitive%20Component%20Object%20Reference) (OtherBodyIndex :type Integer))
  (bind _returnvalue (Actor|GetComponentbyClass OtherActor "/Game/BP_Logic/BP_NPC/BP_DialogueComponent.BP_DialogueComponent_C"))
  (Utilities|IsValid _returnvalue
    (:Is%20Valid
      (Default|EndDialogue _returnvalue self))))

(event EventBeginPlay)

(event Collision|EventActorBeginOverlap
  (params (OtherActor :type Actor%20Object%20Reference)))

(event EventTick
  (params (DeltaSeconds :type Float%20%28single-precision%29)))

(fn ConstructionScript)